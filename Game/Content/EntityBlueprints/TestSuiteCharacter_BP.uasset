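; Test character that exercises Gameplay Ability System activation, effect duration, local prediction and effect removal.
; L runs a timed activate-then-remove cycle locally and through server events; other keys trigger predicted activation by tag or class, or removal alone.
; Tag-based activation and removal, gated by AbilitiesActive, call CheckEffectCount before and after delays to verify effect counts, printing green passes or red failures.
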(event Custom|ActivateAbilities
  (if (not (Variables|Default|GetAbilitiesActive))
    (bind _returnvalue (Abilities|TryActivateAbilitiesbyTag (Variables|Default|GetAbilitySystem) (GameplayTags|MakeGameplayTagContainerfromTag "(TagName=\"GameplayTag.BaseAbility\")") true))
    (if _returnvalue
      (Development|PrintString "Activation succeeded" true true "(R=0.000000,G=1.000000,B=0.000000,A=1.000000)")
      (CallFunction|CheckEffectCount "/Game/GameplayAbility/GE_Duration.GE_Duration_C" 2 "Duration apply")
      (CallFunction|CheckEffectCount "/Game/GameplayAbility/GE_LocalPredicted.GE_LocalPredicted_C" 1 "Local prediction apply")
      (Utilities|FlowControl|Delay 1.6)
      (CallFunction|CheckEffectCount "/Game/GameplayAbility/GE_Duration.GE_Duration_C" 0 "Duration removal")
      (CallFunction|CheckEffectCount "/Game/GameplayAbility/GE_LocalPredicted.GE_LocalPredicted_C" 1 "Local prediction persist")
      (Variables|Default|SetAbilitiesActive true)
      (else
        (Development|PrintString "Activation failed" true true "(R=1.000000,G=0.000000,B=0.000000,A=1.000000)")))))

(event Custom|RemoveActiveEffects
  (if (Variables|Default|GetAbilitiesActive)
    (CallFunction|CheckEffectCount "/Game/GameplayAbility/GE_LocalPredicted.GE_LocalPredicted_C" 1 "Pre removal")
    (GameplayEffects|RemoveActiveEffectswithTags (Variables|Default|GetAbilitySystem) "(GameplayTags=((TagName=\"GameplayTag.BaseEffect\")))")
    (Utilities|FlowControl|Delay 0.2)
    (CallFunction|CheckEffectCount "/Game/GameplayAbility/GE_LocalPredicted.GE_LocalPredicted_C" 0 "Post removal")
    (Variables|Default|SetAbilitiesActive false)))

(event Custom|ServerActivateAbilities
  (CallFunction|ActivateAbilities))

(event Custom|ServerRemoveActiveEffects
  (CallFunction|RemoveActiveEffects))

(event EventTick
  (params (DeltaSeconds :type Float%20%28single-precision%29)))

(event Input|KeyboardEvents|1
  (params (Key :type Key%20Structure))
  (:Released
    (Abilities|TryActivateAbilitiesbyTag (Variables|Default|GetAbilitySystem) (GameplayTags|MakeGameplayTagContainerfromTag "(TagName=\"GameplayTag.LocalPredicted\")") true)))

(event Input|KeyboardEvents|2
  (params (Key :type Key%20Structure))
  (:Released
    (CallFunction|RemoveActiveEffects)))

(event Input|KeyboardEvents|3
  (params (Key :type Key%20Structure))
  (:Released
    (Abilities|TryActivateAbilitybyClass (Variables|Default|GetAbilitySystem) "/Game/GameplayAbility/GA_LocalPredicted.GA_LocalPredicted_C" true)))

(event Input|KeyboardEvents|L
  (params (Key :type Key%20Structure))
  (:Released
    (CallFunction|ActivateAbilities)
    (CallFunction|ServerActivateAbilities)
    (Utilities|FlowControl|Delay 2.0)
    (CallFunction|RemoveActiveEffects)
    (CallFunction|ServerRemoveActiveEffects)))

(fn ConstructionScript)

(fn CheckEffectCount
  (params (Effect :type Gameplay%20Effect%20Class%20Reference) (Count :type Integer) (Fail%20message :type String))
  (if (== (GameplayEffects|GetGameplayEffectCount (Variables|Default|GetAbilitySystem) Effect 0 true) Count)
    (Development|PrintString (Utilities|String|Append "Check passed: " Fail%20message) true true "(R=0.000000,G=1.000000,B=0.000000,A=1.000000)")
    (else
      (Development|PrintString (Utilities|String|Append "Check failed: " Fail%20message) true true "(R=1.000000,G=0.000000,B=0.000000,A=1.000000)"))))